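; BP_Item is a physics-simulated merge item that combines with another BP_Item of identical scale on contact.
; On a Sphere hit with a match, it spawns a double-scale BP_Item at the midpoint of the pair, then destroys both.
; When the doubled X scale would reach the size cap, the pair is destroyed without a replacement.
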(event OnComponentHit(Sphere)
  (params (HitComponent :type Primitive%20Component%20Object%20Reference) (OtherActor :type Actor%20Object%20Reference) (OtherComp :type Primitive%20Component%20Object%20Reference) (NormalImpulse :type Vector :default "0, 0, 0") (Hit :type Hit%20Result%20Structure%20%28by%20ref%29))
  (bind _returnvalue (Transformation|GetActorScale3D))
  (bind _returnvalue_2 (* _returnvalue 2.0))
  (bind _asbp_item (Utilities|Casting|CastToBP_Item OtherActor))
  (if (Utilities|Operators|EqualEqual (Transformation|GetActorScale3D _asbp_item) _returnvalue 0.0)
    (if (>= (.X (Math|Vector|BreakVector _returnvalue_2)) 2.0)
      _
      (else
        (bind _newparam (CallFunction|GetCentralLocation OtherActor))
        (Game|SpawnActorfromClass "BP_Item_C" (Math|Transform|MakeTransform _newparam "0, 0, 0" _returnvalue_2) "Undefined" "MultiplyWithRoot" 0 "NewEnumerator0" 0)))
    (Actor|DestroyActor OtherActor)
    (Actor|DestroyActor)))

(event EventBeginPlay
  (Physics|SetSimulatePhysics (Variables|Default|GetSphere) true))

(fn ConstructionScript)

(fn GetCentralLocation
  (params (Other%20Actor :type Actor%20Object%20Reference))
  (return (/ (+ (Transformation|GetActorLocation) (Transformation|GetActorLocation Other%20Actor)) 2)))